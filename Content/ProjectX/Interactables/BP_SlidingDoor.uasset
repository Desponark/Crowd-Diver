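; BP_SlidingDoor is an interactable sliding door that players toggle through a prompt and NPCs open by entering its trigger box.
; IsClosed changes fire a RepNotify that calls OpenDoor or CloseDoor, with paired DoOnce gates preventing repeat triggers.
; A Timeline played forward or in reverse drives a morph target, switches collision at the halfway point and clears the IsRunning interaction lock when finished.
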(event OnComponentBeginOverlap(TriggerBox)
  (params (OverlappedComponent :type Primitive%20Component%20Object%20Reference) (OtherActor :type Actor%20Object%20Reference) (OtherComp :type Primitive%20Component%20Object%20Reference) (OtherBodyIndex :type Integer) (bFromSweep :type Boolean) (SweepResult :type Hit%20Result%20Structure%20%28by%20ref%29))
  (Utilities|Casting|CastToBP_NPC OtherActor)
  (Variables|Default|SetIsClosed false))

(event Custom|OpenDoor
  (bind _doorcollision (Variables|Default|GetDoorCollision))
  (Utilities|FlowControl|DoOnce false
    (:Completed
      (Utilities|FlowControl|Sequence
        (:then_0
          (bind (_direction _newtrack_1) (Timeline|Timeline Play)
            (:Update
              (Components|SkeletalMesh|SetMorphTarget (Variables|Default|GetSlidingDoor_2) "Key 1" _newtrack_1 true)
              (switch Utilities|FlowControl|Switch|SwitchonETimelineDirection _direction
                (:Forward
                  (if (> _newtrack_1 0.5)
                    (Collision|SetCollisionEnabled _doorcollision "NoCollision")))
                (:Backward
                  (if (< _newtrack_1 0.5)
                    (Collision|SetCollisionEnabled _doorcollision "QueryAndPhysics")))))
            (:Finished
              (Variables|Default|SetIsRunning false))))
        (:then_1
          (Audio|PlaySoundatLocation "/Game/ProjectX/Sounds/Waves/Environmental/ClosingDoor_Cue.ClosingDoor_Cue" (Transformation|GetActorLocation) "0, 0, 0" 1.0 1.0 0.0 0 0 0 0))
        (:then_2
          (Utilities|FlowControl|DoOnce false) ; enters at Reset
        )))))

(event Custom|CloseDoor
  (bind _doorcollision (Variables|Default|GetDoorCollision))
  (Utilities|FlowControl|DoOnce false
    (:Completed
      (Utilities|FlowControl|Sequence
        (:then_0
          (bind (_direction _newtrack_1) (Timeline|Timeline Reverse)
            (:Update
              (Components|SkeletalMesh|SetMorphTarget (Variables|Default|GetSlidingDoor_2) "Key 1" _newtrack_1 true)
              (switch Utilities|FlowControl|Switch|SwitchonETimelineDirection _direction
                (:Forward
                  (if (> _newtrack_1 0.5)
                    (Collision|SetCollisionEnabled _doorcollision "NoCollision")))
                (:Backward
                  (if (< _newtrack_1 0.5)
                    (Collision|SetCollisionEnabled _doorcollision "QueryAndPhysics")))))
            (:Finished
              (Variables|Default|SetIsRunning false))))
        (:then_1
          (Audio|PlaySoundatLocation "/Game/ProjectX/Sounds/Waves/Environmental/ClosingDoor_Cue.ClosingDoor_Cue" (Transformation|GetActorLocation) "0, 0, 0" 1.0 1.0 0.0 0 0 0 0))
        (:then_2
          (Utilities|FlowControl|DoOnce false) ; enters at Reset
        )))))

(event EventOnInteraction
  (params (InteractingPlayer :type Actor%20Object%20Reference))
  (if (not (Variables|Default|GetIsRunning))
    (Variables|Default|SetIsRunning true)
    (Variables|Default|SetIsClosed (not (Variables|Default|GetIsClosed)))))

(fn ConstructionScript)

(fn OnRepIsClosed
  (if (Variables|Default|GetIsClosed)
    (CallFunction|CloseDoor)
    (else
      (CallFunction|OpenDoor))))

(fn InteractionPromptData
  (params (Player%20Controller :type Player%20Controller%20Object%20Reference))
  (return (Utilities|Text|ToText(String) (Utilities|String|SelectString "Press to open" "Press to Close" (Variables|Default|GetIsClosed))) "/Game/ProjectX/MaterialLibrary/UserInterfaceMaterials/Icons/MAT_INST_E_Key.MAT_INST_E_Key" (Variables|Default|GetPromptAnchor)))

(fn IsInteractionDisabled
  (params (PlayerController :type Player%20Controller%20Object%20Reference))
  (return false))
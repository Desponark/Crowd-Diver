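; BP_CalloutArea is a box volume that shows a named area callout on the local player's HUD.
; The construction script sizes the collider from ColliderSize, and BeginPlay caches the ProjectX HUD and blanks its area name.
; When a locally controlled Monster or Seeker begins overlapping, it sends its Name to the HUD; leaving the volume does not clear it.
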(event Collision|EventActorBeginOverlap
  (params (OtherActor :type Actor%20Object%20Reference))
  (bind _asbp_monster (Utilities|Casting|CastToBP_Monster OtherActor)
    (:then
      (if (Pawn|IsLocallyControlled _asbp_monster)
        (Default|SetAreaName (Variables|Default|GetPlayerHud) (Variables|Default|GetName) :!label _label)))
    (:CastFailed
      (bind _asbp_seeker (Utilities|Casting|CastToBP_Seeker OtherActor))
      (if (Pawn|IsLocallyControlled _asbp_seeker)
        (goto _label)))))

(event EventBeginPlay
  (bind _asbp_project_xhud (Utilities|Casting|CastToBP_ProjectXHUD (HUD|GetHUD (Game|GetPlayerController 0))))
  (bind _output_get (Variables|Default|SetPlayerHud _asbp_project_xhud))
  (Default|SetAreaName _output_get))

(fn ConstructionScript
  (Components|Box|SetBoxExtent (Variables|Default|GetCollider) (Variables|Default|GetColliderSize) true))
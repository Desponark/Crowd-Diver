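; Security console interactable that Seekers activate with a hold interaction and the Monster deactivates with a single interaction.
; Seeker movement is locked during the hold, and each state change is reported to the game state.
; The IsActive RepNotify plays a sound, switches the light between blue and red, and drives the nanite swarm spawn rate.
; Prompt text varies by player role, while the role-based disable check is left unconnected.
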(event Custom|StopNaniteVfx
  (Niagara|SetNiagaraVariable(Float) (Variables|Default|GetPS_MeshSwarm) "SpawnRate" 0.0))

(event EventOnInteractionHold
  (params (InteractingPlayer :type Actor%20Object%20Reference))
  ;[1 1 1] Seeker Interaction
  (bind _asbp_seeker (Utilities|Casting|CastToBP_Seeker InteractingPlayer))
  (if (not (Variables|Default|GetIsActive))
    (Pawn|Components|CharacterMovement|SetMovementMode (Variables|/Script/Engine.Character|GetCharacterMovement _asbp_seeker) "MOVE_Walking" 0)
    (Default|ReceiveHoldInteraction _asbp_seeker)
    (Variables|Default|SetIsActive true)
    (Default|UpdateSecurityConsoles (Variables|Default|GetGameState) self)))

(event EventOnInteractionHoldStarted
  (params (InteractingPlayer :type Actor%20Object%20Reference))
  ;[1 1 1] Seeker Interaction
  (bind _asbp_seeker (Utilities|Casting|CastToBP_Seeker InteractingPlayer))
  (if (not (Variables|Default|GetIsActive))
    (Pawn|Components|CharacterMovement|DisableMovement (Variables|/Script/Engine.Character|GetCharacterMovement _asbp_seeker))
    (Default|ReceiveHoldInteractionStarted _asbp_seeker)))

(event EventOnInteractionHoldCanceled
  (params (InteractingPlayer :type Actor%20Object%20Reference))
  ;[1 1 1] Seeker Interaction
  (bind _asbp_seeker (Utilities|Casting|CastToBP_Seeker InteractingPlayer))
  (Pawn|Components|CharacterMovement|SetMovementMode (Variables|/Script/Engine.Character|GetCharacterMovement _asbp_seeker) "MOVE_Walking" 0)
  (Default|ReceiveHoldInteractionCanceled _asbp_seeker))

(event EventOnInteraction
  (params (InteractingPlayer :type Actor%20Object%20Reference))
  ;[1 1 1] Monster Interaction
  (Utilities|Casting|CastToBP_Monster InteractingPlayer)
  (if (Variables|Default|GetIsActive)
    (Variables|Default|SetIsActive false)
    (Default|UpdateSecurityConsoles (Variables|Default|GetGameState) self)))

(event EventBeginPlay
  (Variables|Default|SetGameState (.AsBP%20Project%20XGame%20State%20Base (Utilities|Casting|CastToBP_ProjectXGameStateBase (Game|GetGameState)))))

(event EventInteractionPrompt
  (params (KeepAlive :type Float%20%28double-precision%29) (PlayerController :type Player%20Controller%20Object%20Reference)))

(fn ConstructionScript
  (Variables|Default|SetIsActive (Variables|Default|GetIsActive)))

(fn OnRepIsActive
  (bind _pointlight (Variables|Default|GetPointLight))
  (Audio|PlaySoundatLocation "/Game/ProjectX/Sounds/Waves/Seeker/BindRod/SuckIn.SuckIn" (Transformation|GetActorLocation) "0, 0, 0" 1.0 1.0 0.0 0 0 0 0)
  (if (Variables|Default|GetIsActive)
    (Rendering|Components|Light|SetLightColor _pointlight "(R=0.000000,G=0.000000,B=1.000000,A=1.000000)" true)
    (CallFunction|StopNaniteVfx)
    (else
      (Rendering|Components|Light|SetLightColor _pointlight "(R=1.000000,G=0.000000,B=0.000000,A=1.000000)" true)
      (Niagara|SetNiagaraVariable(Float) (Variables|Default|GetPS_MeshSwarm) "SpawnRate" 5e+01)
      (Utilities|Time|SetTimerbyEvent (EventDispatchers|CreateEvent :!event Custom|StopNaniteVfx) 5.0))))

(fn InteractionPromptData
  (params (Player%20Controller :type Player%20Controller%20Object%20Reference))
  (return (Utilities|Text|ToText(String) (Utilities|String|SelectString "Activate Console" "Hack Console" (Utilities|Enum|Equal(Enum) (Variables|/Game/ProjectX/Core/PlayerStates/BP_ProjectXPlayerState.BP_ProjectXPlayerState_C|GetPlayerRole (.AsBP%20Project%20XPlayer%20State (Utilities|Casting|CastToBP_ProjectXPlayerState (Variables|/Script/Engine.Controller|GetPlayerState Player%20Controller)))) "NewEnumerator2"))) "/Game/ProjectX/MaterialLibrary/UserInterfaceMaterials/Icons/MAT_INST_E_Key.MAT_INST_E_Key" (Variables|Default|GetPromptAnchor)))

(fn IsInteractionDisabled
  (params (PlayerController :type Player%20Controller%20Object%20Reference)))
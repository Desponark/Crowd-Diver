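; BP_NPC is a roaming character that Monster players can kill, either as a marked target or an ordinary NPC.
; It loops AIMoveTo to random reachable points, pausing between moves and retrying on failure.
; Monster interaction starts a timed swarm kill, then plays a sound, destroys the NPC and updates player and game-state kill tallies.
; Custom depth provides target highlighting; Seeker interaction only prints placeholder text.
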(event Custom|MoveNPC
  ;[1 1 1] AI_Random_Roam
  (Variables|Default|SetIsMoving true)
  (AI|AIMoveTo self (.RandomLocation (AI|Navigation|GetRandomReachablePointinRadius (Transformation|GetActorLocation) 2e+03 0 0)) 0 5e+01 true
    (:OnSuccess
      (Variables|Default|SetIsMoving false)
      (Utilities|FlowControl|Delay (Math|Random|RandomFloatinRange 1.0 5.0))
      (CallFunction|MoveNPC))
    (:OnFail
      (Variables|Default|SetIsMoving false)
      (Utilities|FlowControl|Delay 0.2)
      (CallFunction|MoveNPC))))

(event Custom|HighlightAsTarget
  (params (IsHighlighted :type Boolean))
  ;[1 1 1] Set Targets for Monsters
  (Rendering|SetRenderCustomDepth (Variables|Character|GetMesh) IsHighlighted))

(event Custom|PlaySoundReplicated
  (params (Location :type Vector))
  (Audio|PlaySoundatLocation "/Game/ProjectX/Sounds/Waves/Monster/monster-kill-placeholder.monster-kill-placeholder" (Transformation|GetActorLocation) "0, 0, 0" 1.0 1.0 0.0 "/Game/ProjectX/Sounds/Attenuations/ATT_BaseFallOff.ATT_BaseFallOff" 0 0 0))

(event EventBeginPlay
  (CallFunction|MoveNPC))

(event EventOnInteraction
  (params (InteractingPlayer :type Actor%20Object%20Reference))
  (bind _returnvalue (Game|GetGameState))
  (bind _returnvalue_2 (Game|GetInstigatorController InteractingPlayer))
  (bind _asbp_monster (Utilities|Casting|CastToBP_Monster InteractingPlayer))
  (bind _lengthtokill (Variables|Default|GetLengthToKill))
  (bind _asbp_project_xgame_state_base (Utilities|Casting|CastToBP_ProjectXGameStateBase _returnvalue))
  (bind _playerstate (Variables|/Script/Engine.Controller|GetPlayerState _returnvalue_2))
  (bind _asbp_project_xplayer_state (Utilities|Casting|CastToBP_ProjectXPlayerState _playerstate))
  (switch Utilities|FlowControl|Switch|SwitchonEPlayerRole (Variables|/Game/ProjectX/Core/PlayerStates/BP_ProjectXPlayerState.BP_ProjectXPlayerState_C|GetPlayerRole _asbp_project_xplayer_state)
    (:NewEnumerator1
      (if (not (Variables|Default|GetBeingKilled))
        (Default|SetMonsterMovement _asbp_monster true)
        (Default|ActivateSwarm _asbp_monster (Variables|Default|GetLengthToKill) self)
        (Variables|Default|SetBeingKilled true)
        (Default|DisplayNotifyTimerText (.AsBP%20Project%20XPlayer%20Controller (Utilities|Casting|CastToBP_ProjectXPlayerController _returnvalue_2)) _lengthtokill)
        (Utilities|FlowControl|Delay _lengthtokill)
        (Variables|Default|SetBeingKilled false)
        (Default|SetMonsterMovement _asbp_monster false)
        (CallFunction|PlaySoundReplicated "0, 0, 0")
        (if (Variables|Default|GetIsTarget)
          (Actor|DestroyActor)
          (Math|Integer|IncrementInt (Variables|/Game/ProjectX/Core/PlayerStates/BP_ProjectXPlayerState.BP_ProjectXPlayerState_C|GetTargetsKilled _asbp_project_xplayer_state)
            (:%20%20
              (Math|Integer|IncrementInt (Variables|/Game/ProjectX/Core/GameStates/BP_ProjectXGameStateBase.BP_ProjectXGameStateBase_C|GetTotalTargetsKilled _asbp_project_xgame_state_base))))
          (else
            (Actor|DestroyActor)
            (Math|Integer|IncrementInt (Variables|/Game/ProjectX/Core/PlayerStates/BP_ProjectXPlayerState.BP_ProjectXPlayerState_C|GetNPCsKilled _asbp_project_xplayer_state)
              (:%20%20
                (Math|Integer|IncrementInt (Variables|/Game/ProjectX/Core/GameStates/BP_ProjectXGameStateBase.BP_ProjectXGameStateBase_C|GetTotalNPCsKilled _asbp_project_xgame_state_base))))))))
    (:NewEnumerator2
      (Development|PrintText "Seeker interaction (supposed to fail the game)"))))

(fn ConstructionScript)

(fn OnRepIsTarget)

(fn IsInteractable
  (return false))
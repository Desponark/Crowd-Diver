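; Demo NPC character that roams randomly and can be killed, either as a monster's target or as an ordinary NPC.
; The construction script randomizes hair, head, top and bottom meshes from NPC mesh data.
; An AI move loop picks nearby reachable points, pausing between moves and retrying on failure.
; Death updates player and game state kill counts, then ragdolls; targets can be highlighted via custom depth, while interaction is stubbed out.
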(event Custom|MoveNPC
  ;[1 1 1] AI_Random_Roam
  (Variables|Default|SetIsMoving true)
  (AI|AIMoveTo self (.RandomLocation (AI|Navigation|GetRandomReachablePointinRadius (Transformation|GetActorLocation) 2e+03 0 0)) 0 5e+01 true
    (:OnSuccess
      (Variables|Default|SetIsMoving false)
      (Utilities|FlowControl|Delay (Math|Random|RandomFloatinRange 1.0 5.0))
      (CallFunction|MoveNPC))
    (:OnFail
      (Variables|Default|SetIsMoving false)
      (Utilities|FlowControl|Delay 0.2)
      (CallFunction|MoveNPC))))

(event Custom|HighlightAsTarget
  (params (IsHighlighted :type Boolean))
  ;[1 1 1] Set Targets for Monsters
  (Rendering|SetRenderCustomDepth (Variables|Character|GetMesh) IsHighlighted))

(event Custom|PlaySoundAtLocation
  (params (Sound :type Sound%20Base%20Object%20Reference))
  (Audio|PlaySoundatLocation Sound (Transformation|GetActorLocation) "0, 0, 0" 1.0 1.0 0.0 "/Game/ProjectX/Sounds/Attenuations/ATT_BaseFallOff.ATT_BaseFallOff" 0 0 0))

(event Custom|Ragdoll
  (Class|SkeletalMeshComponent|SetAllBodiesSimulatePhysics (Variables|Character|GetMesh) true)
  (Collision|SetCollisionEnabled (Variables|Collision|GetCapsuleComponent) "NoCollision")
  (Collision|SetCollisionEnabled (Variables|Character|GetMesh) "PhysicsOnly"))

(event Custom|GetKilled
  (params (PlayerState :type BP%20Project%20X%20Player%20State%20Object%20Reference))
  (bind _returnvalue (Game|GetGameState))
  (bind _asbp_project_xgame_state_base (Utilities|Casting|CastToBP_ProjectXGameStateBase _returnvalue))
  (if (Variables|Default|GetIsTarget)
    (Math|Integer|IncrementInt (Variables|/Game/ProjectX/Core/PlayerStates/BP_ProjectXPlayerState.BP_ProjectXPlayerState_C|GetTargetsKilled PlayerState)
      (:%20%20
        (Math|Integer|IncrementInt (Variables|/Game/ProjectX/Core/GameStates/BP_ProjectXGameStateBase.BP_ProjectXGameStateBase_C|GetTotalTargetsKilled _asbp_project_xgame_state_base)
          (:%20%20
            (Utilities|Array|RemoveItem (Variables|/Game/ProjectX/Core/GameStates/BP_ProjectXGameStateBase.BP_ProjectXGameStateBase_C|GetKillTargets _asbp_project_xgame_state_base) self)))))
    (else
      (Math|Integer|IncrementInt (Variables|/Game/ProjectX/Core/PlayerStates/BP_ProjectXPlayerState.BP_ProjectXPlayerState_C|GetNPCsKilled PlayerState)
        (:%20%20
          (Math|Integer|IncrementInt (Variables|/Game/ProjectX/Core/GameStates/BP_ProjectXGameStateBase.BP_ProjectXGameStateBase_C|GetTotalNPCsKilled _asbp_project_xgame_state_base)
            (:%20%20
              _))))))
  (CallFunction|Ragdoll))

(event EventBeginPlay
  (CallFunction|MoveNPC))

(event EventOnInteraction
  (params (InteractingPlayer :type Actor%20Object%20Reference)))

(fn ConstructionScript
  (bind _npcmeshdata (Variables|Default|GetNPCMeshData))
  ;[1 1 1] Go to Struc (NPC) and fill in new Assets
  (CallFunction|SkeletonMeshRandomizer (Utilities|GetRandomArrayItem (.hairs _npcmeshdata)) (Utilities|GetRandomArrayItem (.heads _npcmeshdata)) (Utilities|GetRandomArrayItem (.tops _npcmeshdata)) (Utilities|GetRandomArrayItem (.bottoms _npcmeshdata))))

(fn OnRepIsTarget)

(fn SkeletonMeshRandomizer
  (params (SM_Hair :type Skeletal%20Mesh%20Object%20Reference) (SM_Head :type Skeletal%20Mesh%20Object%20Reference) (SM_Top :type Skeletal%20Mesh%20Object%20Reference) (SM_Bottom :type Skeletal%20Mesh%20Object%20Reference))
  (Utilities|FlowControl|Sequence
    (:then_0
      (Components|SkeletalMesh|SetSkeletalMeshAsset (Variables|Character|GetMesh) SM_Head))
    (:then_1
      (Components|SkeletalMesh|SetSkeletalMeshAsset (Variables|Default|GetTop) SM_Top))
    (:then_2
      (Components|SkeletalMesh|SetSkeletalMeshAsset (Variables|Default|GetBottom) SM_Bottom))
    (:then_3
      (Components|SkeletalMesh|SetSkeletalMeshAsset (Variables|Default|GetTest_Wolfcut) SM_Hair))))

(fn InteractionPromptData
  (return "" 0))

(fn IsInteracable
  (return false))

(fn SetIsInteractable
  (params (IsInteractable :type Boolean))
  (return))
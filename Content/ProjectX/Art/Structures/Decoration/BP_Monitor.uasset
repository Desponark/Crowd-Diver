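; BP_Monitor is a decorative holographic monitor that switches on when a BP_Seeker comes near and off when it leaves.
; It starts off, with the HoloMonitor mesh's "Key 1" morph target at full weight.
; Box overlaps toggle IsOn and drive one timeline, reversed from its end on entry and played forward on exit, to animate that morph weight.
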(event OnComponentBeginOverlap(Box)
  (params (OverlappedComponent :type Primitive%20Component%20Object%20Reference) (OtherActor :type Actor%20Object%20Reference) (OtherComp :type Primitive%20Component%20Object%20Reference) (OtherBodyIndex :type Integer) (bFromSweep :type Boolean) (SweepResult :type Hit%20Result%20Structure%20%28by%20ref%29))
  (if (not (Variables|Default|GetIsOn))
    (Utilities|Casting|CastToBP_Seeker OtherActor)
    (Variables|Default|SetIsOn true)
    (bind _monitoron (Timeline|Timeline ReverseFromEnd)
      (:Update
        (Components|SkeletalMesh|SetMorphTarget (Variables|Default|GetHoloMonitor) "Key 1" _monitoron true)))))

(event OnComponentEndOverlap(Box)
  (params (OverlappedComponent :type Primitive%20Component%20Object%20Reference) (OtherActor :type Actor%20Object%20Reference) (OtherComp :type Primitive%20Component%20Object%20Reference) (OtherBodyIndex :type Integer))
  (if (Variables|Default|GetIsOn)
    (Utilities|Casting|CastToBP_Seeker OtherActor)
    (Variables|Default|SetIsOn false)
    (bind _monitoron (Timeline|Timeline Play)
      (:Update
        (Components|SkeletalMesh|SetMorphTarget (Variables|Default|GetHoloMonitor) "Key 1" _monitoron true)))))

(event EventBeginPlay
  (Variables|Default|SetIsOn false)
  (Components|SkeletalMesh|SetMorphTarget (Variables|Default|GetHoloMonitor) "Key 1" 1.0 true))

(event Collision|EventActorBeginOverlap
  (params (OtherActor :type Actor%20Object%20Reference)))

(event EventTick
  (params (DeltaSeconds :type Float%20%28single-precision%29)))

(fn ConstructionScript)
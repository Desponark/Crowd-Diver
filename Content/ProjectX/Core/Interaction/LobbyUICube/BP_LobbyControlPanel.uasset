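; Interactable control panel for the lobby that opens a lobby UI state on the interacting player's HUD.
; Prompt calls refresh a keep-alive timestamp and enable a custom depth stencil highlight, which Tick clears shortly after the calls stop.
; Interaction resolves the player's controller and HUD to set that state, while prompt data supplies the text, key icon and anchor.
; The interactable query always returns false and its setter is empty.
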(event Custom|Call%20UI
  (params (InteractingPlayer :type Actor%20Object%20Reference))
  (bind _asbp_project_xlobby_hud (Utilities|Casting|CastToBP_ProjectXLobbyHUD (HUD|GetHUD (.AsBP%20Project%20XPlayer%20Controller (Utilities|Casting|CastToBP_ProjectXPlayerController (Game|GetInstigatorController InteractingPlayer))))))
  (Default|SetLobbyUIState _asbp_project_xlobby_hud "NewEnumerator3"))

(event EventTick
  (params (DeltaSeconds :type Float%20%28single-precision%29))
  (bind _controlpanel (Variables|Default|GetControlPanel))
  (if (< (+ (Variables|Default|GetKeep%20Alive) 0.075) (Class|KismetMathLibrary|ToUnixTimestampDouble (Math|DateTime|UTCNow)))
    (Rendering|SetRenderCustomDepth _controlpanel false)
    (Rendering|SetCustomDepthStencilValue _controlpanel 1)))

(event EventOnInteraction
  (params (InteractingPlayer :type Actor%20Object%20Reference))
  (CallFunction|CallUI InteractingPlayer))

(event EventInteractionPrompt
  (params (KeepAlive :type Float%20%28double-precision%29) (PlayerController :type Player%20Controller%20Object%20Reference))
  (bind _controlpanel (Variables|Default|GetControlPanel))
  (Variables|Default|SetKeep%20Alive KeepAlive)
  (Rendering|SetRenderCustomDepth _controlpanel true)
  (Rendering|SetCustomDepthStencilValue _controlpanel 2))

(fn ConstructionScript)

(fn InteractionPromptData
  (params (Player%20Controller :type Player%20Controller%20Object%20Reference))
  (return "PRESS TO OPEN" "/Game/ProjectX/Art/UI/Images/PromptIcons/E-KEY.E-KEY" (Variables|Default|GetPromptAnchor)))

(fn IsInteracable
  (return false))

(fn SetIsInteractable
  (params (IsInteractable :type Boolean))
  (return))
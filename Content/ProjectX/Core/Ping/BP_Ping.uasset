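; BP_Ping is a temporary ping marker actor that announces itself with a sound and shows the player's distance to it.
; On BeginPlay it plays the ping cue at its location, waits ten seconds, then destroys itself.
; Each tick it writes the distance to the first player character into the WBP_Ping widget on its Widget component.
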(event EventBeginPlay
  (Audio|PlaySoundatLocation "/Game/ProjectX/Sounds/Waves/Environmental/Ping_Cue.Ping_Cue" (Transformation|GetActorLocation) "0, 0, 0" 1.0 1.0 0.0 0 0 0 0)
  (Utilities|FlowControl|Delay 1e+01)
  (Actor|DestroyActor))

(event EventTick
  (params (DeltaSeconds :type Float%20%28single-precision%29))
  (bind _aswbp_ping (Utilities|Casting|CastToWBP_Ping (UserInterface|GetWidget (Variables|Default|GetWidget))))
  (Variables|/Game/ProjectX/Core/Ping/WBP_Ping.WBP_Ping_C|SetDistance _aswbp_ping (Math|Vector|Distance(Vector) (Transformation|GetActorLocation) (Transformation|GetActorLocation (Game|GetPlayerCharacter 0)))))

(fn ConstructionScript)
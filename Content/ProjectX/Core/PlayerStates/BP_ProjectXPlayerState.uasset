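; Player state for ProjectX that holds each player's role, user ID and username, carrying role and ID across level transitions through CopyProperties.
; On BeginPlay the authority requests the username from Steam, falling back to the local platform user name.
; The PlayerRole RepNotify increments the game state's Monster or Seeker count on authority.
; IsLocallyControlled compares this state against player state index 0.
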(event Custom|SetUsername
  (params (Username :type Text))
  (Variables|Default|SetUsername Username))

(event Custom|RetrieveUsername
  (Networking|SwitchHasAuthority
    (:Authority
      (Development|PrintString (Class|AdvancedSessionsLibrary|UniqueNetIdtoString (Class|AdvancedSessionsLibrary|GetUniqueNetIDfromPlayerState self)) true true "(R=1.000000,G=0.366735,B=0.000000,A=1.000000)" 6e+01)
      (bind _returnvalue (Class|AdvancedSteamFriendsLibrary|RequestSteamFriendInfo :bRequireNameOnly true))
      (if _returnvalue
        (bind _returnvalue_2 (Class|AdvancedSteamFriendsLibrary|GetSteamPersonaName (Class|AdvancedSessionsLibrary|GetUniqueNetIDfromPlayerState self))) ; Requires Request Steam Friend Info if not a friend
        (CallFunction|SetUsername (Utilities|Text|ToText(String) _returnvalue_2))
        (else
          (CallFunction|SetUsername (Utilities|Text|ToText(String) (Utilities|String|Append "Local PC Name: " (Utilities|Platform|GetPlatformUserName)))))))))

(event EventBeginPlay
  (CallFunction|RetrieveUsername))

(event EventCopyProperties
  (params (NewPlayerState :type Player%20State%20Object%20Reference))
  ;[1 1 1] Retain player state between level transitions
  (bind _asbp_project_xplayer_state (Utilities|Casting|CastToBP_ProjectXPlayerState NewPlayerState))
  (Variables|BP_ProjectXPlayerState_C|SetPlayerRole _asbp_project_xplayer_state (Variables|Default|GetPlayerRole))
  (Variables|BP_ProjectXPlayerState_C|SetUserID _asbp_project_xplayer_state (Variables|Default|GetUserID)))

(fn ConstructionScript)

(fn OnRepPlayerRole
  (bind _returnvalue (Game|GetGameState))
  (bind _asbp_project_xgame_state_base (Utilities|Casting|CastToBP_ProjectXGameStateBase _returnvalue))
  (Networking|SwitchHasAuthority
    (:Authority
      (switch Utilities|FlowControl|Switch|SwitchonEPlayerRole (Variables|Default|GetPlayerRole)
        (:NewEnumerator1
          (Math|Integer|IncrementInt (Variables|/Game/ProjectX/Core/GameStates/BP_ProjectXGameStateBase.BP_ProjectXGameStateBase_C|GetMonsterAmount _asbp_project_xgame_state_base)))
        (:NewEnumerator2
          (Math|Integer|IncrementInt (Variables|/Game/ProjectX/Core/GameStates/BP_ProjectXGameStateBase.BP_ProjectXGameStateBase_C|GetSeekerAmount _asbp_project_xgame_state_base)))))))

(fn OnRepID)

(fn IsLocallyControlled
  (return (== self (Game|GetPlayerState 0))))
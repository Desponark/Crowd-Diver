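; Base GameState for ProjectX that keeps lobby player listings in sync and passes the match round count along.
; UpdateSelectionLeaderboard copies PlayerArray into the RepNotify variable AllPlayerStates, whose OnRep refreshes player listings on every lobby menu and lobby HUD widget.
; SetTotalRounds stores the value on BP_OnlineGameInstance, while the TotalRounds OnRep here is empty.
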(event Custom|UpdateSelectionLeaderboard
  (Variables|Default|SetAllPlayerStates (Variables|Default|GetPlayerArray)))

(event Custom|Set%20Total%20Rounds
  (params (Total%20Rounds :type Integer))
  (Variables|/Game/ProjectX/Core/GameInstance/BP_OnlineGameInstance.BP_OnlineGameInstance_C|SetTotalRounds (.AsBP%20Online%20Game%20Instance (Utilities|Casting|CastToBP_OnlineGameInstance (Game|GetGameInstance))) Total%20Rounds))

(fn ConstructionScript)

(fn OnRepAllPlayerStates
  (Utilities|FlowControl|Sequence
    (:then_0
      (bind _foundwidgets (Widget|GetAllWidgetsOfClass "/Game/ProjectX/Core/UI/WBP_LobbyMenu.WBP_LobbyMenu_C" false))
      (for _array_element _foundwidgets
        (Default|UpdatePlayerListingWidget _array_element)))
    (:then_1
      (bind _foundwidgets_2 (Widget|GetAllWidgetsOfClass "/Game/ProjectX/Core/UI/WBP_LobbyHUD.WBP_LobbyHUD_C" false))
      (for _array_element_2 _foundwidgets_2
        (Default|UpdatePlayerListingWidget _array_element_2)))))

(fn OnRepTotalRounds)
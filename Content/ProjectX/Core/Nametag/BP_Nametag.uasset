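; BP_Nametag is an actor that shows a player's username above their pawn, visible only when the local player shares the instigating player's role.
; BeginPlay compares roles, then either fills the WBP_Nametag text and records the starting camera distance or hides the component hierarchy.
; Tick follows the pawn at a height offset, using camera distance relative to that start to make the tag more opaque and smaller when farther, within clamps.
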(event EventBeginPlay
  (bind _returnvalue (Game|GetPlayerController 0))
  (bind _playerstate (Variables|/Script/Engine.Controller|GetPlayerState _returnvalue))
  (bind _asbp_project_xplayer_state (Utilities|Casting|CastToBP_ProjectXPlayerState _playerstate))
  ;[1 1 1] Check if instigating player is same role as local player and show ping or not
  (Utilities|IsValid _asbp_project_xplayer_state
    (:Is%20Valid
      (if (Utilities|Enum|Equal(Enum) (Variables|/Game/ProjectX/Core/PlayerStates/BP_ProjectXPlayerState.BP_ProjectXPlayerState_C|GetPlayerRole _asbp_project_xplayer_state) (Variables|Default|GetInstigatingPlayerRole))
        (Variables|/Script/UMG.TextBlock|SetText (Variables|/Game/ProjectX/Core/UI/Widgets/Nametag/WBP_Nametag.WBP_Nametag_C|GetName (.AsWBP%20Nametag (Utilities|Casting|CastToWBP_Nametag (UserInterface|GetWidget (Variables|Default|GetNametag))))) (Variables|Default|GetUsername))
        (Variables|Default|SetStart%20Distance (Math|Vector|Distance(Vector) (Transformation|GetActorLocation) (Camera|GetCameraLocation (Game|GetPlayerCameraManager 0))))
        (else
          (Rendering|SetVisibility (Variables|Default|GetDefaultSceneRoot) false true))))))

(event EventTick
  (params (DeltaSeconds :type Float%20%28single-precision%29))
  (bind _returnvalue (Transformation|GetActorLocation))
  (bind _returnvalue_2 (Game|GetPlayerCameraManager 0))
  (bind _start_distance (Variables|Default|GetStart%20Distance))
  (bind _pawn (Variables|Default|GetPawn))
  (bind _returnvalue_3 (Camera|GetCameraLocation _returnvalue_2))
  (bind _returnvalue_4 (Math|Vector|Distance(Vector) _returnvalue _returnvalue_3))
  (bind _returnvalue_5 (/ _returnvalue_4 _start_distance))
  (bind _returnvalue_6 (* _returnvalue_5 2.0))
  (bind _returnvalue_7 (- 1.3 _returnvalue_6))
  (bind _returnvalue_8 (Math|Float|Clamp(Float) _returnvalue_7 0.65 1.0))
  (if (Utilities|IsValid _pawn)
    (Transformation|SetWorldLocation (Variables|Default|GetDefaultSceneRoot) (+ (Transformation|GetActorLocation _pawn) "0.000000,0.000000,100.000000") false false)
    (bind _aswbp_nametag (Utilities|Casting|CastToWBP_Nametag (UserInterface|GetWidget (Variables|Default|GetNametag))))
    (Widget|SetRenderOpacity _aswbp_nametag (Math|Float|Clamp(Float) (+ 0.1 _returnvalue_6) 0.0 0.85))
    (Widget|Transform|SetRenderScale _aswbp_nametag (Math|Vector2D|MakeVector2D _returnvalue_8 _returnvalue_8))))

(fn ConstructionScript)
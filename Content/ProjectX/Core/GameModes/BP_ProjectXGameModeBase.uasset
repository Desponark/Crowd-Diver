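; Game mode for a Monsters vs Seekers round match, spawning each player's pawn by role.
; BeginPlay picks random NPC kill targets, reveals them to Monsters and starts a countdown, copied to GameState via RepNotify.
; Tick checks GameState kill totals and time to show game over, then after a delay restarts via ServerTravel or returns to Lobby after the last round.
; Login and logout maintain the controller list and refresh the leaderboard.
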(event Custom|Update%20Player%20List
  ;[1 1 1] Player List
  (Utilities|FlowControl|Delay 0.3)
  (bind _asbp_project_xgame_state_base (Utilities|Casting|CastToBP_ProjectXGameStateBase (Game|GetGameState)))
  (Default|UpdateSelectionLeaderboard _asbp_project_xgame_state_base))

(event Custom|RestartLevel
  ;[1 1 1] Restart Level
  (bind _returnvalue (Game|GetCurrentLevelName true))
  (Development|PrintString (Utilities|String|Append "ServerTravel " _returnvalue))
  (Development|ExecuteConsoleCommand (Utilities|String|Append "ServerTravel " _returnvalue) 0))

(event EventBeginPlay
  (Utilities|FlowControl|Sequence
    (:then_0
      ;[1 1 1] Select 3 NPCs and make them kill targets
      (bind _outactors (Actor|GetAllActorsOfClass "/Game/ProjectX/Characters/NPC/BP_NPC.BP_NPC_C"))
      (if (>= (Utilities|Array|Length _outactors) (Variables|Default|GetMaxTargets))
        (while (< (Utilities|Array|Length (Variables|Default|GetKillTargets)) (Variables|Default|GetMaxTargets))
          (if (Utilities|IsValid (.OutItem (Utilities|Array|Random _outactors)))
            (Utilities|Array|AddUnique (Variables|Default|GetKillTargets) (.OutItem (Utilities|Array|Random _outactors)))
            (Variables|Default|SetKillTargets (Variables|Default|GetKillTargets))))
        (for _array_element (Variables|Default|GetKillTargets)
          (bind _asbp_npc (Utilities|Casting|CastToBP_NPC _array_element))
          (Variables|/Game/ProjectX/Characters/NPC/BP_NPC.BP_NPC_C|SetIsTarget _asbp_npc true))))
    (:then_1
      ;[1 1 1] Game Timer
      (Utilities|Time|SetTimerbyFunctionName 0 "DecrementTimeLimit" 1.0 true))
    (:then_2
      ;[1 1 1] PlayerList
      (CallFunction|UpdatePlayerList))
    (:then_3
      (for _index (range 0 (Class|GameplayStatics|GetNumPlayerControllers))
        (bind _asbp_project_xplayer_controller (Utilities|Casting|CastToBP_ProjectXPlayerController (Game|GetPlayerController _index)))
        (bind _asbp_project_xplayer_state (Utilities|Casting|CastToBP_ProjectXPlayerState (Variables|/Script/Engine.Controller|GetPlayerState (Game|GetPlayerController _index))))
        (switch Utilities|FlowControl|Switch|SwitchonEPlayerRole (Variables|/Game/ProjectX/Core/PlayerStates/BP_ProjectXPlayerState.BP_ProjectXPlayerState_C|GetPlayerRole _asbp_project_xplayer_state)
          (:NewEnumerator1
            (Default|MakeKillTargetsVisible _asbp_project_xplayer_controller)))))))

(event EventTick
  (params (DeltaSeconds :type Float%20%28single-precision%29))
  (bind _returnvalue (Game|GetGameInstance))
  (bind _returnvalue_2 (Game|GetGameState))
  (bind _asbp_project_xgame_state_base (Utilities|Casting|CastToBP_ProjectXGameStateBase _returnvalue_2))
  (bind _asbp_online_game_instance (Utilities|Casting|CastToBP_OnlineGameInstance _returnvalue))
  (bind _totalmonsterskilled (Variables|/Game/ProjectX/Core/GameStates/BP_ProjectXGameStateBase.BP_ProjectXGameStateBase_C|GetTotalMonstersKilled _asbp_project_xgame_state_base))
  ;[1 1 1] Check for win or lose
  (Utilities|FlowControl|Sequence
    (:then_0
      ;;[1 1 1] Monster Won
      (if (>= (Variables|/Game/ProjectX/Core/GameStates/BP_ProjectXGameStateBase.BP_ProjectXGameStateBase_C|GetTotalTargetsKilled _asbp_project_xgame_state_base) (Variables|Default|GetMaxTargets))
        (CallFunction|ShowGameOverScreentoAllPlayers "Monsters have Won!")
        ;;[1 1 1] Check Rounds
        (Utilities|FlowControl|Delay 4.0 :!label _label)
        (if (< (Variables|/Game/ProjectX/Core/GameInstance/BP_OnlineGameInstance.BP_OnlineGameInstance_C|GetCurrentRound _asbp_online_game_instance) (Variables|/Game/ProjectX/Core/GameInstance/BP_OnlineGameInstance.BP_OnlineGameInstance_C|GetTotalRounds _asbp_online_game_instance))
          (Variables|/Game/ProjectX/Core/GameInstance/BP_OnlineGameInstance.BP_OnlineGameInstance_C|SetCurrentRound _asbp_online_game_instance (+ (Variables|/Game/ProjectX/Core/GameInstance/BP_OnlineGameInstance.BP_OnlineGameInstance_C|GetCurrentRound _asbp_online_game_instance) 1))
          (CallFunction|RestartLevel)
          (else
            (CallFunction|TraveltoLobby)
            (Variables|/Game/ProjectX/Core/GameInstance/BP_OnlineGameInstance.BP_OnlineGameInstance_C|SetCurrentRound _asbp_online_game_instance 1)))))
    (:then_1
      ;;[1 1 1] Seekers Won
      (if (and (> _totalmonsterskilled 0) (>= _totalmonsterskilled (Variables|/Game/ProjectX/Core/GameStates/BP_ProjectXGameStateBase.BP_ProjectXGameStateBase_C|GetMonsterAmount _asbp_project_xgame_state_base)))
        (CallFunction|ShowGameOverScreentoAllPlayers "Seekers have Won!")
        (goto _label)))
    (:then_2
      ;;[1 1 1] Time Limit Over
      (if (<= (Variables|Default|GetTimeLimit) 0)
        (CallFunction|ShowGameOverScreentoAllPlayers "Time Limit Over!")
        (goto _label)))))

(event EventPostLogin
  (params (NewPlayer :type Player%20Controller%20Object%20Reference))
  ;[1 1 1] Player List
  (bind _asbp_project_xplayer_controller (Utilities|Casting|CastToBP_ProjectXPlayerController NewPlayer))
  (bind _asbp_project_xgame_state_base (Utilities|Casting|CastToBP_ProjectXGameStateBase (Game|GetGameState)))
  (Utilities|Array|Add (Variables|Default|GetAllPlayerControllers) _asbp_project_xplayer_controller)
  (Variables|/Game/ProjectX/Core/PlayerStates/BP_ProjectXPlayerState.BP_ProjectXPlayerState_C|SetUserID (stale EventOnLogout _asbp_project_xplayer_state) (+ (Variables|/Game/ProjectX/Core/GameStates/BP_ProjectXGameStateBase.BP_ProjectXGameStateBase_C|GetOnID _asbp_project_xgame_state_base) 1))
  (CallFunction|UpdatePlayerList))

(event EventOnLogout
  (params (ExitingController :type Controller%20Object%20Reference))
  ;[1 1 1] Player List
  (bind _asbp_project_xplayer_controller (Utilities|Casting|CastToBP_ProjectXPlayerController ExitingController))
  (Utilities|Array|RemoveItem (Variables|Default|GetAllPlayerControllers) _asbp_project_xplayer_controller)
  (bind _asbp_project_xplayer_state (Utilities|Casting|CastToBP_ProjectXPlayerState (Variables|/Script/Engine.Controller|GetPlayerState _asbp_project_xplayer_controller)))
  (Variables|/Game/ProjectX/Core/PlayerStates/BP_ProjectXPlayerState.BP_ProjectXPlayerState_C|SetUserID _asbp_project_xplayer_state (- (Variables|/Game/ProjectX/Core/GameStates/BP_ProjectXGameStateBase.BP_ProjectXGameStateBase_C|GetOnID (stale EventPostLogin _asbp_project_xgame_state_base)) 1))
  (CallFunction|UpdatePlayerList))

(fn ConstructionScript)

(fn OnRepTimeLimit
  (Variables|/Game/ProjectX/Core/GameStates/BP_ProjectXGameStateBase.BP_ProjectXGameStateBase_C|SetTimeLimit (.AsBP%20Project%20XGame%20State%20Base (Utilities|Casting|CastToBP_ProjectXGameStateBase (Game|GetGameState))) (Variables|Default|GetTimeLimit)))

(fn OnRepKillTargets
  (Variables|/Game/ProjectX/Core/GameStates/BP_ProjectXGameStateBase.BP_ProjectXGameStateBase_C|SetKillTargets (.AsBP%20Project%20XGame%20State%20Base (Utilities|Casting|CastToBP_ProjectXGameStateBase (Game|GetGameState))) (Variables|Default|GetKillTargets)))

(fn DecrementTimeLimit
  (bind _result (Math|Integer|DecrementInt (Variables|Default|GetTimeLimit))
    (:%20%20
      (Variables|Default|SetTimeLimit _result))))

(fn ShowGameOverScreentoAllPlayers
  (params (Message :type String))
  (for _array_element (Variables|/Script/Engine.GameStateBase|GetPlayerArray (Game|GetGameState))
    (Default|ShowGameOverScreen (.AsBP%20Project%20XPlayer%20Controller (Utilities|Casting|CastToBP_ProjectXPlayerController (Game|GetPlayerController _array_element))) Message)))

(fn GetDefaultPawnClassforController
  (params (InController :type Controller%20Object%20Reference))
  (switch Utilities|FlowControl|Switch|SwitchonEPlayerRole (Variables|/Game/ProjectX/Core/PlayerStates/BP_ProjectXPlayerState.BP_ProjectXPlayerState_C|GetPlayerRole (.AsBP%20Project%20XPlayer%20State (Utilities|Casting|CastToBP_ProjectXPlayerState (Variables|/Script/Engine.Controller|GetPlayerState InController))))
    (:NewEnumerator1
      (return "/Game/ProjectX/Characters/Monster/BP_Monster.BP_Monster_C"))
    (:NewEnumerator2
      (return "/Game/ProjectX/Characters/Seeker/BP_Seeker.BP_Seeker_C"))))

(fn TraveltoLobby
  (bind _returnvalue (Utilities|String|Append "ServerTravel " "Lobby"))
  (Development|PrintString _returnvalue)
  (Development|ExecuteConsoleCommand _returnvalue 0))

(fn UpdateSelectionLeaderboard)
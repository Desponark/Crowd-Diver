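; Player controller for a Monster-versus-Seeker game that assigns a role and spawns and possesses the matching pawn.
; Hit events run short forward line traces: Seekers destroy Monsters, Monsters destroy NPCs, distinguishing targets from bystanders.
; Each kill increments counters on the attacker's PlayerState and the GameState.
; It also creates the game-over screen with a message and highlights the GameState's kill targets.
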(event Custom|SERVERSpawnPawn
  (params (PlayerRole :type EPlayerRole%20Enum :default "NewEnumerator0"))
  (bind _returnvalue (Math|Transform|MakeTransform "0, 0, 0"))
  ;[1 1 1] Spawn Pawn depending on Role
  (switch Utilities|FlowControl|Switch|SwitchonEPlayerRole PlayerRole
    (:NewEnumerator1
      (bind _returnvalue_2 (Game|SpawnActorfromClass "/Game/ProjectX/Characters/Monster/BP_Monster.BP_Monster_C" _returnvalue "Undefined" "MultiplyWithRoot" 0 0))
      (Pawn|Possess _returnvalue_2))
    (:NewEnumerator2
      (bind _returnvalue_3 (Game|SpawnActorfromClass "/Game/ProjectX/Characters/Seeker/BP_Seeker.BP_Seeker_C" _returnvalue "Undefined" "MultiplyWithRoot" 0 0))
      (Pawn|Possess _returnvalue_3))))

(event Custom|ShowGameOverScreen
  (params (Message :type String))
  (bind _returnvalue (UserInterface|CreateWidget "/Game/ProjectX/Core/UI/WBP_GameOver.WBP_GameOver_C"))
  (Variables|/Script/UMG.TextBlock|SetText (Variables|/Game/ProjectX/Core/UI/WBP_GameOver.WBP_GameOver_C|GetTextBlock_Message _returnvalue) (Utilities|Text|ToText(String) Message))
  (UserInterface|Viewport|AddtoViewport _returnvalue 0))

(event Custom|ShowTargetHighlights
  (for _array_element (Variables|/Game/ProjectX/Core/GameModes/BP_ProjectXGameStateBase.BP_ProjectXGameStateBase_C|GetKillTargets (.AsBP%20Project%20XGame%20State%20Base (Utilities|Casting|CastToBP_ProjectXGameStateBase (Game|GetGameState))))
    (bind _asbp_npc (Utilities|Casting|CastToBP_NPC _array_element))
    (Default|HightlightasTarget _asbp_npc true)))

(event Custom|SetPlayerRole
  (params (PlayerRole :type EPlayerRole%20Enum :default "NewEnumerator0"))
  (bind _output_get (Variables|/Game/ProjectX/Core/GameModes/BP_ProjectXPlayerState.BP_ProjectXPlayerState_C|SetPlayerRole (.AsBP%20Project%20XPlayer%20State (Utilities|Casting|CastToBP_ProjectXPlayerState (Variables|GetPlayerState))) PlayerRole))
  (CallFunction|SERVERSpawnPawn _output_get))

(event Custom|SeekerHitTarget
  (params (Actor :type BP%20Seeker%20Object%20Reference))
  (bind _returnvalue (Transformation|GetActorTransform Actor))
  (bind _outhit (Collision|LineTraceForObjects (.location _returnvalue) (+ (.location _returnvalue) (* (Math|Vector|GetForwardVector (.rotation _returnvalue)) 3e+02)) (Utilities|Array|MakeArray "ObjectTypeQuery3") false (Utilities|Array|MakeArray Actor) "ForDuration"))
  (bind _asbp_monster (Utilities|Casting|CastToBP_Monster (.hitactor _outhit)))
  (Actor|DestroyActor _asbp_monster)
  (Math|Integer|IncrementInt (Variables|/Game/ProjectX/Core/GameModes/BP_ProjectXPlayerState.BP_ProjectXPlayerState_C|GetMonstersKilled (.AsBP%20Project%20XPlayer%20State (Utilities|Casting|CastToBP_ProjectXPlayerState (Variables|/Script/Engine.Pawn|GetPlayerState Actor))))
    (:%20%20
      (Math|Integer|IncrementInt (Variables|/Game/ProjectX/Core/GameModes/BP_ProjectXGameStateBase.BP_ProjectXGameStateBase_C|GetTotalMonstersKilled (.AsBP%20Project%20XGame%20State%20Base (Utilities|Casting|CastToBP_ProjectXGameStateBase (Game|GetGameState))))))))

(event Custom|MonsterHitTarget
  (params (MonsterPawn :type BP%20Monster%20Object%20Reference))
  (bind _returnvalue (Game|GetGameState))
  (bind _returnvalue_2 (Transformation|GetActorTransform MonsterPawn))
  (bind _playerstate (Variables|/Script/Engine.Pawn|GetPlayerState MonsterPawn))
  (bind _asbp_project_xplayer_state (Utilities|Casting|CastToBP_ProjectXPlayerState _playerstate))
  (bind _asbp_project_xgame_state_base (Utilities|Casting|CastToBP_ProjectXGameStateBase _returnvalue))
  (bind _outhit (Collision|LineTraceForObjects (.location _returnvalue_2) (+ (.location _returnvalue_2) (* (Math|Vector|GetForwardVector (.rotation _returnvalue_2)) 3e+02)) (Utilities|Array|MakeArray "ObjectTypeQuery3") false (Utilities|Array|MakeArray MonsterPawn) "ForDuration"))
  (bind _asbp_npc (Utilities|Casting|CastToBP_NPC (.hitactor _outhit)))
  (if (Variables|/Game/ProjectX/Characters/NPC/BP_NPC.BP_NPC_C|GetIsTarget _asbp_npc)
    (Actor|DestroyActor _asbp_npc)
    (Math|Integer|IncrementInt (Variables|/Game/ProjectX/Core/GameModes/BP_ProjectXPlayerState.BP_ProjectXPlayerState_C|GetTargetsKilled _asbp_project_xplayer_state)
      (:%20%20
        (Math|Integer|IncrementInt (Variables|/Game/ProjectX/Core/GameModes/BP_ProjectXGameStateBase.BP_ProjectXGameStateBase_C|GetTotalTargetsKilled _asbp_project_xgame_state_base))))
    (else
      (Actor|DestroyActor _asbp_npc)
      (Math|Integer|IncrementInt (Variables|/Game/ProjectX/Core/GameModes/BP_ProjectXPlayerState.BP_ProjectXPlayerState_C|GetNPCsKilled _asbp_project_xplayer_state)
        (:%20%20
          (Math|Integer|IncrementInt (Variables|/Game/ProjectX/Core/GameModes/BP_ProjectXGameStateBase.BP_ProjectXGameStateBase_C|GetTotalNPCsKilled _asbp_project_xgame_state_base)))))))

(event EventBeginPlay)

(event EventTick
  (params (DeltaSeconds :type Float%20%28single-precision%29)))

(fn ConstructionScript)
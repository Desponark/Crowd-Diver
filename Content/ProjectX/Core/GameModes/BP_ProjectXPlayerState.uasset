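; Player state for ProjectX that feeds each player's role and kill stats into match-wide counters on BP_ProjectXGameStateBase.
; RepNotify on PlayerRole increments the game state's Monster or Seeker head count.
; RepNotifies for NPC, monster and target kills each add one to the matching total, regardless of the replicated value.
; All logic lives in these notifies, with no active event graph.
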(event EventBeginPlay)

(event EventTick
  (params (DeltaSeconds :type Float%20%28single-precision%29)))

(fn ConstructionScript)

(fn OnRepPlayerRole
  (bind _returnvalue (Game|GetGameState))
  (bind _asbp_project_xgame_state_base (Utilities|Casting|CastToBP_ProjectXGameStateBase _returnvalue))
  (switch Utilities|FlowControl|Switch|SwitchonEPlayerRole (Variables|Default|GetPlayerRole)
    (:NewEnumerator1
      (Math|Integer|IncrementInt (Variables|/Game/ProjectX/Core/GameModes/BP_ProjectXGameStateBase.BP_ProjectXGameStateBase_C|GetMonsterAmount _asbp_project_xgame_state_base)))
    (:NewEnumerator2
      (Math|Integer|IncrementInt (Variables|/Game/ProjectX/Core/GameModes/BP_ProjectXGameStateBase.BP_ProjectXGameStateBase_C|GetSeekerAmount _asbp_project_xgame_state_base)))))

(fn OnRepNPCsKilled
  (Math|Integer|IncrementInt (Variables|/Game/ProjectX/Core/GameModes/BP_ProjectXGameStateBase.BP_ProjectXGameStateBase_C|GetTotalNPCsKilled (.AsBP%20Project%20XGame%20State%20Base (Utilities|Casting|CastToBP_ProjectXGameStateBase (Game|GetGameState))))))

(fn OnRepMonstersKilled
  (Math|Integer|IncrementInt (Variables|/Game/ProjectX/Core/GameModes/BP_ProjectXGameStateBase.BP_ProjectXGameStateBase_C|GetTotalMonstersKilled (.AsBP%20Project%20XGame%20State%20Base (Utilities|Casting|CastToBP_ProjectXGameStateBase (Game|GetGameState))))))

(fn OnRepTargetsKilled
  (Math|Integer|IncrementInt (Variables|/Game/ProjectX/Core/GameModes/BP_ProjectXGameStateBase.BP_ProjectXGameStateBase_C|GetTotalTargetsKilled (.AsBP%20Project%20XGame%20State%20Base (Utilities|Casting|CastToBP_ProjectXGameStateBase (Game|GetGameState))))))
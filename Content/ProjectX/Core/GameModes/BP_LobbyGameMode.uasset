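; Lobby game mode for ProjectX that tracks joining and leaving players and picks their pawn class by role.
; Login and logout update the game state's Players array and refresh every controller's player list; login also stores the array index as UserID.
; BeginPlay triggers the game state's leaderboard update after a short delay.
; The default pawn override maps PlayerRole to third-person character, Monster or Seeker.
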(event Custom|UpdateSelectionLeaderboard
  (bind _outactors (Actor|GetAllActorsOfClass "/Game/ProjectX/Core/Controllers/BP_ProjectXPlayerController.BP_ProjectXPlayerController_C"))
  (for _array_element _outactors
    (Default|UpdatePlayerList _array_element)
    (Development|PrintText (Utilities|Text|ToText(Object) _array_element))))

(event EventBeginPlay
  (Utilities|FlowControl|Delay 0.75)
  (bind _asbp_project_xgame_state_base (Utilities|Casting|CastToBP_ProjectXGameStateBase (Game|GetGameState)))
  (Default|UpdateSelectionLeaderboard _asbp_project_xgame_state_base))

(event EventTick
  (params (DeltaSeconds :type Float%20%28single-precision%29)))

(event EventPostLogin
  (params (NewPlayer :type Player%20Controller%20Object%20Reference))
  (bind _asbp_project_xplayer_controller (Utilities|Casting|CastToBP_ProjectXPlayerController NewPlayer))
  (Default|UpdatePlayerList _asbp_project_xplayer_controller)
  (bind _asbp_project_xgame_state_base (Utilities|Casting|CastToBP_ProjectXGameStateBase (Game|GetGameState)))
  (bind _returnvalue (Utilities|Array|Add (Variables|/Game/ProjectX/Core/GameStates/BP_ProjectXGameStateBase.BP_ProjectXGameStateBase_C|GetPlayers _asbp_project_xgame_state_base) (Variables|/Script/Engine.Controller|GetPlayerState _asbp_project_xplayer_controller)))
  (CallFunction|UpdateSelectionLeaderboard)
  (bind _asbp_project_xplayer_state (Utilities|Casting|CastToBP_ProjectXPlayerState (Variables|/Script/Engine.Controller|GetPlayerState _asbp_project_xplayer_controller)))
  (Utilities|IsValid _asbp_project_xplayer_state
    (:Is%20Valid
      (Variables|/Game/ProjectX/Core/PlayerStates/BP_ProjectXPlayerState.BP_ProjectXPlayerState_C|SetUserID _asbp_project_xplayer_state _returnvalue))))

(event EventOnLogout
  (params (ExitingController :type Controller%20Object%20Reference))
  (bind _asbp_project_xplayer_controller (Utilities|Casting|CastToBP_ProjectXPlayerController ExitingController))
  (bind _asbp_project_xgame_state_base (Utilities|Casting|CastToBP_ProjectXGameStateBase (Game|GetGameState)))
  (Utilities|Array|RemoveItem (Variables|/Game/ProjectX/Core/GameStates/BP_ProjectXGameStateBase.BP_ProjectXGameStateBase_C|GetPlayers _asbp_project_xgame_state_base) (Variables|/Script/Engine.Controller|GetPlayerState _asbp_project_xplayer_controller))
  (CallFunction|UpdateSelectionLeaderboard)
  (bind _asbp_project_xplayer_state (Utilities|Casting|CastToBP_ProjectXPlayerState (Variables|/Script/Engine.Controller|GetPlayerState (stale EventPostLogin _asbp_project_xplayer_controller))))
  (Utilities|IsValid _asbp_project_xplayer_state
    (:Is%20Valid
      (Variables|/Game/ProjectX/Core/PlayerStates/BP_ProjectXPlayerState.BP_ProjectXPlayerState_C|SetUserID _asbp_project_xplayer_state (stale EventPostLogin _returnvalue)))))

(event EventEndPlay
  (params (EndPlayReason :type EEndPlayReason%20Enum :default "Destroyed"))
  (Development|PrintString (Utilities|String|EnumtoString EndPlayReason)))

(fn ConstructionScript)

(fn GetDefaultPawnClassforController
  (params (InController :type Controller%20Object%20Reference))
  (switch Utilities|FlowControl|Switch|SwitchonEPlayerRole (Variables|/Game/ProjectX/Core/PlayerStates/BP_ProjectXPlayerState.BP_ProjectXPlayerState_C|GetPlayerRole (.AsBP%20Project%20XPlayer%20State (Utilities|Casting|CastToBP_ProjectXPlayerState (Variables|/Script/Engine.Controller|GetPlayerState InController))))
    (:NewEnumerator0
      (return "/Game/ProjectX/Characters/ThirdPersonCharacter/BP_ThirdPersonCharacter.BP_ThirdPersonCharacter_C"))
    (:NewEnumerator1
      (return "/Game/ProjectX/Characters/Monster/BP_Monster.BP_Monster_C"))
    (:NewEnumerator2
      (return "/Game/ProjectX/Characters/Seeker/BP_Seeker.BP_Seeker_C"))))
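; Placeable ambience sound trigger that plays a configurable sound cue when a character enters its sphere.
; The construction script applies the cue, attenuation settings and sphere radius variables to the audio and collision components.
; On overlap, only BP_ThirdPersonCharacter, BP_Monster or BP_Seeker start playback from the beginning.
; Nothing in the graph guards against retriggering or stops the sound on exit.
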(event OnComponentBeginOverlap(SphereCollision)
  (params (OverlappedComponent :type Primitive%20Component%20Object%20Reference) (OtherActor :type Actor%20Object%20Reference) (OtherComp :type Primitive%20Component%20Object%20Reference) (OtherBodyIndex :type Integer) (bFromSweep :type Boolean) (SweepResult :type Hit%20Result%20Structure%20%28by%20ref%29))
  (Utilities|Casting|CastToBP_ThirdPersonCharacter OtherActor
    (:then
      _)
    (:CastFailed
      (Utilities|Casting|CastToBP_Monster OtherActor
        (:then
          _)
        (:CastFailed
          (Utilities|Casting|CastToBP_Seeker OtherActor)))))
  (Audio|Components|Audio|Play (Variables|Default|GetAmbienceSound) 0.0))

(event EventBeginPlay)

(event Collision|EventActorBeginOverlap
  (params (OtherActor :type Actor%20Object%20Reference)))

(event EventTick
  (params (DeltaSeconds :type Float%20%28single-precision%29)))

(fn ConstructionScript
  (Audio|Components|Audio|SetSound (Variables|Default|GetAmbienceSound) (Variables|Default|GetSoundCue))
  (Variables|/Script/Engine.AudioComponent|SetAttenuationSettings (Variables|Default|GetAmbienceSound) (Variables|Default|GetAmbientSoundAttenuation))
  (Components|Sphere|SetSphereRadius (Variables|Default|GetSphereCollision) (Variables|Default|GetSphereRadius) true))